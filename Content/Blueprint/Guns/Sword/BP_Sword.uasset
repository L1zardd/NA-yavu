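; Sword pickup actor that becomes the player hero's equipped weapon.
; PickUp detaches any item already held in the BP_hero Equip variable, then stores this sword there.
; The sword snaps to the Hand socket on the hero's Sprite component, keeping its relative scale.
; BeginPlay, overlap and Tick are empty, so pickup relies on an external call to PickUp.
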(event `/Game/Blueprint/Guns/Sword/BPI_Interact.PickUp`
  (bind _defaultsceneroot (`self.DefaultSceneRoot`))
  (bind (_returnvalue_x _returnvalue_y _returnvalue_z) (`KismetMathLibrary.BreakVector` (`SceneComponent.K2_GetComponentLocation` _defaultsceneroot)))
  (bind (_returnvalue_roll _returnvalue_pitch _returnvalue_yaw) (`KismetMathLibrary.BreakRotator` (`SceneComponent.K2_GetComponentRotation` _defaultsceneroot)))
  (bind _asbp_hero (cast `/Game/Blueprint/CharacterMain/BP_hero` (`GameplayStatics.GetPlayerCharacter` 0) :!pure true))
  (bind _equip (`/Game/Blueprint/CharacterMain/BP_hero.Equip` (cast `/Game/Blueprint/CharacterMain/BP_hero` (`GameplayStatics.GetPlayerCharacter` 0) :!pure true)))
  (`/Engine/EditorBlueprintResources/StandardMacros.IsValid` _equip
    (:`Is Valid`
      (`self.K2_DetachFromActor` _equip "KeepRelative" "KeepRelative" "KeepRelative")
      (`self.K2_SetActorLocationAndRotation` (`KismetMathLibrary.MakeVector` _returnvalue_x _returnvalue_y _returnvalue_z) (`KismetMathLibrary.MakeRotator` _returnvalue_roll _returnvalue_pitch _returnvalue_yaw)))
    (:`Is Not Valid`
      _))
  (set `/Game/Blueprint/CharacterMain/BP_hero.Equip` self _asbp_hero)
  (`self.K2_AttachToComponent` (`PaperCharacter.Sprite` _asbp_hero) "Hand" "SnapToTarget" "SnapToTarget" "KeepRelative"))

(fn `UserConstructionScript`)